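; BP_WinDevice is a level exit that opens ProtoType_Level as soon as the player character enters its Box.
; The same overlap then increments TransitionCount, or opens MainMenuMap once the count exceeds one.
; An Interact press also opens MainMenuMap while IsPlayerOverlapping is set, and leaving the Box clears that flag and hides the Widget.
; The nodes that set the flag and show the Widget are unwired, leaving that prompt path inactive.
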(event OnComponentBeginOverlap(Box)
  (params (OverlappedComponent :type Primitive%20Component%20Object%20Reference) (OtherActor :type Actor%20Object%20Reference) (OtherComp :type Primitive%20Component%20Object%20Reference) (OtherBodyIndex :type Integer) (bFromSweep :type Boolean) (SweepResult :type Hit%20Result%20Structure%20%28by%20ref%29))
  (if (== OtherActor (Game|GetPlayerCharacter 0))
    (Game|OpenLevel(byName) "ProtoType_Level")
    (if (<= (Variables|Default|GetTransitionCount) 1)
      (Variables|Default|SetTransitionCount (+ (Variables|Default|GetTransitionCount) 1))
      (else
        (Game|OpenLevel(byName) "MainMenuMap")))))

(event OnComponentEndOverlap(Box)
  (params (OverlappedComponent :type Primitive%20Component%20Object%20Reference) (OtherActor :type Actor%20Object%20Reference) (OtherComp :type Primitive%20Component%20Object%20Reference) (OtherBodyIndex :type Integer))
  (if (== OtherActor (Game|GetPlayerCharacter 0))
    (Variables|Default|SetIsPlayerOverlapping false)
    (Rendering|SetVisibility (Variables|Default|GetWidget) false false)))

(event EventBeginPlay
  (Input|EnableInput (Game|GetPlayerController 0)))

(event Input|ActionEvents|InputActionInteract
  (params (Key :type Key%20Structure :default "None"))
  (:Pressed
    (if (Variables|Default|GetIsPlayerOverlapping)
      (Game|OpenLevel(byName) "MainMenuMap"))))

(fn ConstructionScript)