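; PlayMusic_BP is a music player Blueprint that starts a single hard-coded rock workout loop track when play begins.
; BeginPlay calls the PlayNextSong event, which sets that track on the Audio component and plays it from the start.
; Playlist logic using SongList and SongIndex is left disconnected, and the OnAudioFinished event is empty, so the Blueprint never advances to another song.
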(event OnAudioFinished(Audio))

(event Custom|PlayNextSong
  (Audio|Components|Audio|SetSound (Variables|Default|GetAudio) "/Game/FPSAssets/Sounds/Songs/rock-workout-sports-electro-loop-113540.rock-workout-sports-electro-loop-113540")
  (Audio|Components|Audio|Play (Variables|Default|GetAudio) 0.0))

(event EventBeginPlay
  (CallFunction|PlayNextSong))

(event Collision|EventActorBeginOverlap
  (params (OtherActor :type Actor%20Object%20Reference)))

(event EventTick
  (params (DeltaSeconds :type Float%20%28single-precision%29)))

(fn ConstructionScript)