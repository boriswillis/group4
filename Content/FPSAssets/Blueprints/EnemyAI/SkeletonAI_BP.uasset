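; SkeletonAI_BP is a skeleton enemy that handles taking damage and dying.
; AnyDamage subtracts a fixed amount of Health per hit, and non-lethal hits briefly show a hit marker widget with a flesh impact sound.
; At zero Health, a DoOnce plays the death animation, sets IsDead and destroys the actor after a delay.
; Tick polls IsDead to destroy the capsule component during that delay.
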(event EventTick
  (params (DeltaSeconds :type Float%20%28single-precision%29))
  (if (Variables|Default|GetIsDead)
    (Components|DestroyComponent (Variables|Collision|GetCapsuleComponent))))

(event Game|Damage|EventAnyDamage
  (params (Damage :type Float%20%28single-precision%29) (DamageType :type Damage%20Type%20Object%20Reference) (InstigatedBy :type Controller%20Object%20Reference) (DamageCauser :type Actor%20Object%20Reference))
  (bind _output_get (Variables|Default|SetHealth (- (Variables|Default|GetHealth) 2e+01)))
  (if (<= _output_get 0.0)
    (Utilities|FlowControl|DoOnce false
      (:Completed
        (Components|Animation|PlayAnimation (Variables|Character|GetMesh) "/Game/FPSAssets/Blueprints/EnemyAI/SkeletonCharacter/Animations/SkeletonCharacter/ANI_Death_B.ANI_Death_B" false)
        (Variables|Default|SetIsDead true)
        (Utilities|FlowControl|Delay 2.0)
        (Actor|DestroyActor)))
    (else
      (bind _returnvalue (UserInterface|CreateWidget "/Game/FPSAssets/Blueprints/FirstPersonBP/Blueprints/WB_HitMarker.WB_HitMarker_C" (Game|GetPlayerController 0)))
      (UserInterface|Viewport|AddtoPlayerScreen _returnvalue)
      (Utilities|FlowControl|Delay 0.1)
      (Audio|PlaySound2D "/Game/FPSAssets/Sounds/Sound_Packs/Bullet_Impacts_Flybys_Pro/Wavs/Body_Flesh/Body_Flesh_7.Body_Flesh_7" 2.0 1.0 0.0 0 0)
      (Utilities|FlowControl|Delay 0.15)
      (Widget|RemovefromParent _returnvalue))))

(fn ConstructionScript)